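; ParentTile_BP is a parent track tile that chains to others through an AttachPoint transform exposed to callers.
; When a Starlight actor overlaps EndBox, it asks FoSGameMode to add a tile, then destroys itself after a short delay.
; Its construction script runs PlasmaSpawner, which adds a child actor component at a random point inside SpawnZone, with the random count range currently fixed at zero.
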(event `self.EndBox.OnComponentBeginOverlap`
  (params (OverlappedComponent :type "PrimitiveComponent Object Reference") (OtherActor :type "Actor Object Reference") (OtherComp :type "PrimitiveComponent Object Reference") (OtherBodyIndex :type Integer) (bFromSweep :type Boolean) (SweepResult :type "HitResult Structure (by ref)"))
  (cast `/Game/FoSBlueprints/Characters/Starlight` OtherActor)
  (bind _asfo_sgame_mode (cast `/Game/GameMode/FoSGameMode` (`GameplayStatics.GetGameMode`)))
  (`/Game/GameMode/FoSGameMode.AddTile` _asfo_sgame_mode)
  (`KismetSystemLibrary.Delay` 2.0)
  (`self.K2_DestroyActor`))

(fn `GetAttachPointTransform`
  (returns (`Attach Transform` :type "Transform Structure"))
  (return (`SceneComponent.K2_GetComponentToWorld` (`self.AttachPoint`))))

(fn `PlasmaSpawner`
  (bind _spawnzone (`self.SpawnZone`))
  (for _ (range (+ (`KismetMathLibrary.RandomIntegerInRange` 0) 1))
    (`AddComponent|NODE_AddChildActorComponent-1` :`RelativeTransform` (`KismetMathLibrary.Conv_VectorToTransform` (`KismetMathLibrary.RandomPointInBoundingBox` (`SceneComponent.RelativeLocation` _spawnzone) (`BoxComponent.BoxExtent` _spawnzone))))))

(fn `UserConstructionScript`
  (`self.PlasmaSpawner`))